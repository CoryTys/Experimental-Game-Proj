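; PushDownLadder is an interactable ladder that the first-person character pushes down and can then climb.
; The Collider volume enables input and flags the character as in range.
; Pressing F while LookingAtPersp is set destroys that volume and plays a timeline that lerps the ladder to its lowered position.
; Once IsLadderDown is set, Collider2 overlaps toggle the character's OnLadder state, calling NotOnLadder on exit.
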(event `self.Collider2.OnComponentBeginOverlap`
  (params (OverlappedComponent :type "PrimitiveComponent Object Reference") (OtherActor :type "Actor Object Reference") (OtherComp :type "PrimitiveComponent Object Reference") (OtherBodyIndex :type Integer) (bFromSweep :type Boolean) (SweepResult :type "HitResult Structure (by ref)"))
  (if (`self.IsLadderDown`)
    (bind _asbp_first_person_character (cast `/Game/FirstPerson/Blueprints/BP_FirstPersonCharacter` OtherActor))
    (set `/Game/FirstPerson/Blueprints/BP_FirstPersonCharacter.OnLadder` true _asbp_first_person_character)))

(event `self.Collider2.OnComponentEndOverlap`
  (params (OverlappedComponent :type "PrimitiveComponent Object Reference") (OtherActor :type "Actor Object Reference") (OtherComp :type "PrimitiveComponent Object Reference") (OtherBodyIndex :type Integer))
  (if (`self.IsLadderDown`)
    (bind _asbp_first_person_character (cast `/Game/FirstPerson/Blueprints/BP_FirstPersonCharacter` OtherActor))
    (`/Game/FirstPerson/Blueprints/BP_FirstPersonCharacter.NotOnLadder` _asbp_first_person_character)
    (set `/Game/FirstPerson/Blueprints/BP_FirstPersonCharacter.OnLadder` false _asbp_first_person_character)))

(event `self.Collider.OnComponentBeginOverlap`
  (params (OverlappedComponent :type "PrimitiveComponent Object Reference") (OtherActor :type "Actor Object Reference") (OtherComp :type "PrimitiveComponent Object Reference") (OtherBodyIndex :type Integer) (bFromSweep :type Boolean) (SweepResult :type "HitResult Structure (by ref)"))
  (bind _asbp_first_person_character (cast `/Game/FirstPerson/Blueprints/BP_FirstPersonCharacter` OtherActor))
  (set `/Game/FirstPerson/Blueprints/BP_FirstPersonCharacter.InPerspCollider` true _asbp_first_person_character)
  (`self.EnableInput` (`GameplayStatics.GetPlayerController` 0)))

(event `self.Collider.OnComponentEndOverlap`
  (params (OverlappedComponent :type "PrimitiveComponent Object Reference") (OtherActor :type "Actor Object Reference") (OtherComp :type "PrimitiveComponent Object Reference") (OtherBodyIndex :type Integer))
  (bind _asbp_first_person_character (cast `/Game/FirstPerson/Blueprints/BP_FirstPersonCharacter` OtherActor))
  (set `/Game/FirstPerson/Blueprints/BP_FirstPersonCharacter.InPerspCollider` false _asbp_first_person_character)
  (`self.DisableInput` (`GameplayStatics.GetPlayerController` 0)))

(event `Key|F`
  (params (Key :type "Key Structure"))
  (:`Pressed`
    (bind _asbp_first_person_character (cast `/Game/FirstPerson/Blueprints/BP_FirstPersonCharacter` (stale `self.Collider.OnComponentBeginOverlap` OtherActor)))
    (if (`/Game/FirstPerson/Blueprints/BP_FirstPersonCharacter.LookingAtPersp` _asbp_first_person_character)
      (`ActorComponent.K2_DestroyComponent` (`self.Collider`))
      (bind (_direction _lower_ladder) (`Timeline|Timeline` :!via `PlayFromStart`)
        (:`Update`
          (`SceneComponent.K2_SetRelativeLocation` (`self.Ladder`) (`KismetMathLibrary.VLerp` (`self.Ladder up`) (`self.Ladder down`) _lower_ladder) false false)
          (set `self.IsLadderDown` true))))))

(fn `GetCommand`
  (returns (Command :type Text))
  (return (`self.Command`)))

(fn `UserConstructionScript`)