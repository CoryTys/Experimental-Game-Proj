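; Perspective puzzle actor that lets the first-person player toggle between two sets of components while standing in its trigger collider.
; Overlap begin and end set the character's InPerspCollider flag and enable or disable this actor's input.
; Pressing F flips State, swapping visibility and collision between the S1 and S2 component groups so only one is visible and collidable.
; GetName exposes the actor's Name variable.
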(event `self.Collider.OnComponentBeginOverlap`
  (params (OverlappedComponent :type "PrimitiveComponent Object Reference") (OtherActor :type "Actor Object Reference") (OtherComp :type "PrimitiveComponent Object Reference") (OtherBodyIndex :type Integer) (bFromSweep :type Boolean) (SweepResult :type "HitResult Structure (by ref)"))
  (bind _asbp_first_person_character (cast `/Game/FirstPerson/Blueprints/BP_FirstPersonCharacter` OtherActor))
  (set `/Game/FirstPerson/Blueprints/BP_FirstPersonCharacter.InPerspCollider` true _asbp_first_person_character)
  (`self.EnableInput` (`GameplayStatics.GetPlayerController` 0)))

(event `Key|F`
  (params (Key :type "Key Structure"))
  (:`Pressed`
    (if (`self.State`)
      (`SceneComponent.SetVisibility` (`self.S1`) true false)
      (`SceneComponent.SetVisibility` (`self.S1-4`) true false)
      (`SceneComponent.SetVisibility` (`self.S1-3`) true false)
      (`SceneComponent.SetVisibility` (`self.S1-2`) true false)
      (`SceneComponent.SetVisibility` (`self.S1-1`) true false)
      (`PrimitiveComponent.SetCollisionEnabled` (`self.S1`) "QueryAndPhysics")
      (`PrimitiveComponent.SetCollisionEnabled` (`self.S1-4`) "QueryAndPhysics")
      (`PrimitiveComponent.SetCollisionEnabled` (`self.S1-2`) "QueryAndPhysics")
      (`PrimitiveComponent.SetCollisionEnabled` (`self.S1-1`) "QueryAndPhysics")
      (`PrimitiveComponent.SetCollisionEnabled` (`self.S1-3`) "QueryAndPhysics")
      (`SceneComponent.SetVisibility` (`self.S2`) false false)
      (`SceneComponent.SetVisibility` (`self.S2-1`) false false)
      (`SceneComponent.SetVisibility` (`self.S2-2`) false false)
      (`SceneComponent.SetVisibility` (`self.S2-3`) false false)
      (`SceneComponent.SetVisibility` (`self.S2-4`) false false)
      (`PrimitiveComponent.SetCollisionEnabled` (`self.S2`) "NoCollision")
      (`PrimitiveComponent.SetCollisionEnabled` (`self.S2-4`) "NoCollision")
      (`PrimitiveComponent.SetCollisionEnabled` (`self.S2-3`) "NoCollision")
      (`PrimitiveComponent.SetCollisionEnabled` (`self.S2-2`) "NoCollision")
      (`PrimitiveComponent.SetCollisionEnabled` (`self.S2-1`) "NoCollision")
      (set `self.State` false)
      (else
        (`SceneComponent.SetVisibility` (`self.S1`) false false)
        (`SceneComponent.SetVisibility` (`self.S1-1`) false false)
        (`SceneComponent.SetVisibility` (`self.S1-2`) false false)
        (`SceneComponent.SetVisibility` (`self.S1-3`) false false)
        (`SceneComponent.SetVisibility` (`self.S1-4`) false false)
        (`PrimitiveComponent.SetCollisionEnabled` (`self.S1`) "NoCollision")
        (`PrimitiveComponent.SetCollisionEnabled` (`self.S1-1`) "NoCollision")
        (`PrimitiveComponent.SetCollisionEnabled` (`self.S1-2`) "NoCollision")
        (`PrimitiveComponent.SetCollisionEnabled` (`self.S1-3`) "NoCollision")
        (`PrimitiveComponent.SetCollisionEnabled` (`self.S1-4`) "NoCollision")
        (`SceneComponent.SetVisibility` (`self.S2`) true false)
        (`SceneComponent.SetVisibility` (`self.S2-1`) true false)
        (`SceneComponent.SetVisibility` (`self.S2-2`) true false)
        (`SceneComponent.SetVisibility` (`self.S2-3`) true false)
        (`SceneComponent.SetVisibility` (`self.S2-4`) true false)
        (`PrimitiveComponent.SetCollisionEnabled` (`self.S2`) "QueryAndPhysics")
        (`PrimitiveComponent.SetCollisionEnabled` (`self.S2-1`) "QueryAndPhysics")
        (`PrimitiveComponent.SetCollisionEnabled` (`self.S2-2`) "QueryAndPhysics")
        (`PrimitiveComponent.SetCollisionEnabled` (`self.S2-3`) "QueryAndPhysics")
        (`PrimitiveComponent.SetCollisionEnabled` (`self.S2-4`) "QueryAndPhysics")
        (set `self.State` true)))))

(event `self.Collider.OnComponentEndOverlap`
  (params (OverlappedComponent :type "PrimitiveComponent Object Reference") (OtherActor :type "Actor Object Reference") (OtherComp :type "PrimitiveComponent Object Reference") (OtherBodyIndex :type Integer))
  (bind _asbp_first_person_character (cast `/Game/FirstPerson/Blueprints/BP_FirstPersonCharacter` OtherActor))
  (set `/Game/FirstPerson/Blueprints/BP_FirstPersonCharacter.InPerspCollider` false _asbp_first_person_character)
  (`self.DisableInput` (`GameplayStatics.GetPlayerController` 0)))

(fn `GetName`
  (returns (Name :type Text))
  (return (`self.Name`)))

(fn `UserConstructionScript`)